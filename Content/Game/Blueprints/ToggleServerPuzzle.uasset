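; Puzzle actor that unlocks once every server in its ServersToCheck list is switched off.
; The Open/On and Close/Off events share one check, which folds each server's OnOff state into the Solved flag and calls Unlock when all are off.
; Solved then stays true, so later toggles skip the check.
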(event EventBeginPlay)

(event Collision|EventActorBeginOverlap
  (params (OtherActor :type Actor%20Object%20Reference)))

(event EventTick
  (params (DeltaSeconds :type Float%20%28single-precision%29)))

(event EventOpen/On
  (params (HorrorEvent :type Boolean))
  (if (not (Variables|Default|Getsolved))
    (Variables|Default|Setsolved true)
    (for _array_element (Variables|Default|GetServersToCheck)
      (Variables|Default|Setsolved (and (not (Variables|/Game/Game/Blueprints/PoweredServer.PoweredServer_C|GetOn%20/%20Off _array_element)) (Variables|Default|Getsolved))))
    (if (Variables|Default|Getsolved)
      (CallFunction|Unlock false))))

(event EventClose/Off
  (params (HorrorEvent :type Boolean))
  (if (not (Variables|Default|Getsolved))
    (Variables|Default|Setsolved true)
    (for _array_element (Variables|Default|GetServersToCheck)
      (Variables|Default|Setsolved (and (not (Variables|/Game/Game/Blueprints/PoweredServer.PoweredServer_C|GetOn%20/%20Off _array_element)) (Variables|Default|Getsolved))))
    (if (Variables|Default|Getsolved)
      (CallFunction|Unlock false))))

(fn ConstructionScript)